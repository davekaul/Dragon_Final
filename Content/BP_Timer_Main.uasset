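; BP_Timer_Main is the game's countdown controller, deciding between win and lose for the dragon objective.
; Tick keeps playing a timeline until COMPLETE, checking each update for the timer reaching zero (lose) or both NumDragons flags on the first Dragon and Dragon_2ND actors (win).
; Either outcome adds its widget plus a shared game-over widget, then sets COMPLETE.
; A separate OnTimerExpired function only prints a debug string.
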(event EventTick
  (params (DeltaSeconds :type Float%20%28single-precision%29))
  (if (not (Variables|Default|GetCOMPLETE))
    (bind _timer (Timeline|Timer Play)
      (:Update
        (Utilities|FlowControl|Sequence
          (:then_0
            (bind _outactors (Actor|GetAllActorsOfClass "/Game/Dragon.Dragon_C"))
            (if (and (not (Variables|Default|GetCOMPLETE)) (<= _timer 0.0))
              (bind _returnvalue (UserInterface|CreateWidget "/Game/WBP_lose.WBP_lose_C"))
              (UserInterface|Viewport|AddtoViewport _returnvalue 0)
              (bind _returnvalue_2 (UserInterface|CreateWidget "/Game/WBP_GAMEOVER.WBP_GAMEOVER_C" :!label _label))
              (UserInterface|Viewport|AddtoViewport _returnvalue_2 0)
              (Variables|Default|SetCOMPLETE true)))
          (:then_1
            (bind _outactors_2 (Actor|GetAllActorsOfClass "/Game/dragon_2ND.dragon_2ND_C"))
            (if (and (Variables|/Game/Dragon.Dragon_C|GetNumDragons (Utilities|Array|Get(acopy) _outactors)) (and (Variables|/Game/dragon_2ND.dragon_2ND_C|GetNumDragons2 (Utilities|Array|Get(acopy) _outactors_2)) (not (Variables|Default|GetCOMPLETE))))
              (bind _returnvalue_3 (UserInterface|CreateWidget "/Game/WBP_Win.WBP_Win_C"))
              (UserInterface|Viewport|AddtoViewport _returnvalue_3 0)
              (goto _label))))))))

(fn ConstructionScript)

(fn OnTimerExpired
  (Development|PrintString "DEATH"))